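; BP_Ball is a physics-driven ball actor that launches itself when play begins.
; On BeginPlay, it applies an impulse of InitialImpulse scaled by BallSpeed to its Sphere component as a velocity change, so mass is ignored.
; Each Tick prints the sphere's current linear speed to the screen as debug output.
; The overlap event and construction script are empty.
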(event EventBeginPlay
  (Physics|AddImpulse (Variables|Default|GetSphere) (* (Variables|Default|GetInitialImpulse) (Variables|Default|GetBallSpeed)) "None" true))

(event Collision|EventActorBeginOverlap
  (params (OtherActor :type Actor%20Object%20Reference)))

(event EventTick
  (params (DeltaSeconds :type Float%20%28single-precision%29))
  (bind _returnvalue (Physics|GetPhysicsLinearVelocity (Variables|Default|GetSphere) "None"))
  (Development|PrintString (Utilities|String|ToString(Float) (Math|Vector|VectorLength _returnvalue))))

(fn ConstructionScript)