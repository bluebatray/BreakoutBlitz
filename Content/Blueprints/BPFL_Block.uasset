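; Blueprint function library that looks up block properties by tier.
; GetBlockProperties converts the tier to a row name and reads that row from the DT_BlockProperties data table.
; GetColorFromTier and GetNumberOfLevelsFromTier wrap that lookup to return the row's color and level count.
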(fn GetColorfromTier
  (params (Tier :type Integer))
  (bind _blockproperties (CallFunction|GetBlockProperties Tier))
  (return (.LinearColor (Utilities|Struct|BreakS_BlockProperties _blockproperties))))

(fn GetNumberOfLevelsfromTier
  (params (Tier :type Integer))
  (bind _blockproperties (CallFunction|GetBlockProperties Tier))
  (return (.Levels (Utilities|Struct|BreakS_BlockProperties _blockproperties))))

(fn GetBlockProperties
  (params (Tier :type Integer))
  (bind _returnvalue (Utilities|GetDataTableRow "/Game/Data/DT_BlockProperties.DT_BlockProperties" (Utilities|String|StringToName (Utilities|String|ToString(Integer) Tier)))
    (:then
      (return _returnvalue))))