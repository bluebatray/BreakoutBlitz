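; BP_Paddle is a player paddle that slides horizontally along world Y, can be resized, and plays a sound on PaddleHit.
; The Move event offsets it by direction, speed and delta time, then clamps it between hard-coded bounds inset by the paddle's half-width.
; ChangePaddleSize scales the mesh's X relative to the scale cached at BeginPlay, then recalculates half-width and movement limits.
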(event Custom|Move
  (params (MoveX :type Float%20%28double-precision%29))
  (CallFunction|MovePaddleHorizontally MoveX))

(event EventBeginPlay
  (CallFunction|SetBaseScale))

(fn ConstructionScript)

(fn CalculatePaddleHalfWidth
  (Variables|Default|SetfPaddleHalfWidth (/ (* (.x (Transformation|GetWorldScale (Variables|Default|GetPaddle))) 1e+02) 2.0)))

(fn MovePaddleHorizontally
  (params (Direction :type Float%20%28double-precision%29))
  (Transformation|AddActorWorldOffset (Math|Vector|MakeVector 0.0 (* Direction (Variables|Default|GetfPaddleSpeed) (Utilities|Time|GetWorldDeltaSeconds)) 0.0))
  (CallFunction|ClampPaddle))

(fn ChangePaddleSize
  (params (Scale :type Float%20%28double-precision%29))
  (Transformation|SetRelativeScale3D (Variables|Default|GetPaddle) (Math|Vector|MakeVector (* Scale (Variables|Default|GetfBaseScale)) 1.0 1.0))
  (CallFunction|CalculatePaddleHalfWidth)
  (CallFunction|CalculatePaddleLimits))

(fn SetBaseScale
  (Variables|Default|SetfBaseScale (.x (Variables|/Script/Engine.SceneComponent|GetRelativeScale3D (Variables|Default|GetPaddle)))))

(fn CalculatePaddleLimits
  (Variables|Default|SetfPaddleMoveLimitLow (+ (Variables|Default|GetfPaddleHalfWidth) -1.25e+04))
  (Variables|Default|SetfPaddleMoveLimitHigh (- 7.35e+03 (Variables|Default|GetfPaddleHalfWidth))))

(fn PaddleHit
  (CallFunction|PlaySound "NewEnumerator2"))

(fn ClampPaddle
  (bind _returnvalue (Transformation|GetActorLocation))
  (Transformation|SetActorLocation (Math|Vector|MakeVector (.x _returnvalue) (Math|Float|Clamp(Float) (.y _returnvalue) (Variables|Default|GetfPaddleMoveLimitLow) (Variables|Default|GetfPaddleMoveLimitHigh)) (.z _returnvalue)) false false))