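; Blueprint function library of shared core helpers for a Breakout game, wrapping access to its Game Instance and Game Mode.
; UpdateGameState stores the new state on the Game Instance, then calls the matching Game Mode state-change handler for main menu, playing, paused or game over.
; Other helpers reset the Game Instance for a new game and add the Game Mode's level time to its total game time.
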(fn GetBreakoutGameInstance
  (bind _asbp_breakout_game_instance (Utilities|Casting|CastToBP_BreakoutGameInstance (Game|GetGameInstance)))
  (return _asbp_breakout_game_instance))

(fn GetBreakoutGameMode
  (bind _asbp_breakout_game_mode (Utilities|Casting|CastToBP_BreakoutGameMode (Game|GetGameMode)))
  (return _asbp_breakout_game_mode))

(fn UpdateGameState
  (params (NewGameState :type E_GameState%20Enum :default "NewEnumerator0"))
  (bind _asbp_breakout_game_instance (CallFunction|GetBreakoutGameInstance))
  (Variables|/Game/Blueprints/Core/BP_BreakoutGameInstance.BP_BreakoutGameInstance_C|SeteCurrentGameState _asbp_breakout_game_instance NewGameState)
  (bind _breakout_game_mode (CallFunction|GetBreakoutGameMode))
  (LocalVariables|SetGameMode _breakout_game_mode)
  (switch Utilities|FlowControl|Switch|SwitchonE_GameState NewGameState
    (:NewEnumerator0
      (Default|StateChangeEnterMainMenu (LocalVariables|GetGameMode)))
    (:NewEnumerator1
      (Default|StateChangeEnterPlayingGame (LocalVariables|GetGameMode)))
    (:NewEnumerator2
      (Default|StateChangeEnterPause (LocalVariables|GetGameMode)))
    (:NewEnumerator3
      (Default|StateChangeEnterGameOver (LocalVariables|GetGameMode)))))

(fn InitGame
  (bind _asbp_breakout_game_instance (CallFunction|GetBreakoutGameInstance))
  (Default|ResetAll _asbp_breakout_game_instance))

(fn AddLevelTimetoTotal
  (bind _breakout_game_mode (CallFunction|GetBreakoutGameMode))
  (bind _asbp_breakout_game_instance (CallFunction|GetBreakoutGameInstance))
  (Default|AddtoTotalGameTime _asbp_breakout_game_instance (Variables|/Game/Blueprints/Core/BP_BreakoutGameMode.BP_BreakoutGameMode_C|GetfLevelTime _breakout_game_mode)))