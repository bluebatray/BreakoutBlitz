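; Blueprint function library that plays sound effects and music in the Breakout game from enum values.
; GetSound uses the enum's name as a row name in DT_Sounds, returning the row's Sound Cue if valid and its source sound otherwise.
; PlaySound plays the resolved asset as 2D audio, while PlayMusic passes it to the MusicManager on the Breakout game mode.
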(fn PlaySound
  (params (Sound :type E_Sounds%20Enum :default "NewEnumerator0"))
  (bind _out_row_sound_source (CallFunction|GetSound Sound))
  (Audio|PlaySound2D 0 _out_row_sound_source 1.0 1.0 0.0 0 0)
  (return))

(fn PlayMusic
  (params (Music :type E_Sounds%20Enum :default "NewEnumerator0"))
  (bind _out_row_sound_source (CallFunction|GetSound Music))
  (Default|PlayMusic (Variables|/Game/Blueprints/Core/BP_BreakoutGameMode.BP_BreakoutGameMode_C|GetMusicManager (CallFunction|GetBreakoutGameMode)) _out_row_sound_source)
  (return))

(fn GetSound
  (params (SoundEnum :type E_Sounds%20Enum :default "NewEnumerator0"))
  (bind _returnvalue (Utilities|GetDataTableRow "/Game/Data/DT_Sounds.DT_Sounds" (Utilities|String|StringToName (Utilities|String|EnumtoString SoundEnum)))
    (:then
      ;[0 0 0] If Sound cue exists, use it, otherwise use sound
      (if (Utilities|IsValid (.soundcue _returnvalue))
        (return (.soundcue _returnvalue))
        (else
          (return (.soundsource _returnvalue)))))))