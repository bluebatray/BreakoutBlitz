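; Function library for the Breakout game's save slots, storing and retrieving high score lists per difficulty.
; Easy, Normal and Hard each map to a slot enum value, whose string form is the save slot name.
; AddHighScore appends to the loaded BP_HighScoreSave, or creates one if loading fails.
; It loads by the passed difficulty but saves under the game instance's current difficulty.
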(fn LoadSlot
  (params (Slot :type E_Slots%20Enum :default "NewEnumerator0"))
  (bind _returnvalue (SaveGame|DoesSaveGameExist (Utilities|String|EnumtoString Slot)))
  (if _returnvalue
    (bind _returnvalue_2 (SaveGame|LoadGamefromSlot (Utilities|String|EnumtoString Slot)))
    (return _returnvalue_2 true)
    (else
      (return 0 false))))

(fn GetHighScores
  (params (Difficulty :type E_Difficulties%20Enum :default "NewEnumerator0"))
  (bind (_success _slotdata) (CallFunction|LoadDifficultySlot 0 Difficulty))
  (if _success
    (bind _asbp_high_score_save (Utilities|Casting|CastToBP_HighScoreSave _slotdata))
    (return _asbp_high_score_save true)
    (else
      (return 0 false))))

(fn AddHighScore
  (params (Difficulty :type E_Difficulties%20Enum :default "NewEnumerator0") (NewHighScore :type S%20High%20Score%20Structure))
  (bind (_asbp_high_score_save _success) (CallFunction|GetHighScores Difficulty))
  (if _success
    ;[0 0 0] Add new one to array
    (bind _returnvalue (Utilities|Array|Add (Variables|/Game/Blueprints/BP_HighScoreSave.BP_HighScoreSave_C|GetHighScores _asbp_high_score_save) NewHighScore))
    (CallFunction|SaveHighScore (Variables|/Game/Blueprints/Core/BP_BreakoutGameInstance.BP_BreakoutGameInstance_C|GeteCurrentDifficulty (CallFunction|GetBreakoutGameInstance)) _asbp_high_score_save)
    (Development|PrintText 0 (Utilities|Text|FormatText "added new high score to list {index}" _returnvalue) true true "(R=0.000000,G=0.660000,B=1.000000,A=1.000000)" 2e+01)
    (else
      ;[0 0 0] No high scores saved, create blank and save
      (bind _returnvalue_2 (SaveGame|CreateSaveGameObject "/Game/Blueprints/BP_HighScoreSave.BP_HighScoreSave_C"))
      (Variables|/Game/Blueprints/BP_HighScoreSave.BP_HighScoreSave_C|SetHighScores _returnvalue_2 (Utilities|Array|MakeArray NewHighScore))
      (CallFunction|SaveHighScore (Variables|/Game/Blueprints/Core/BP_BreakoutGameInstance.BP_BreakoutGameInstance_C|GeteCurrentDifficulty (CallFunction|GetBreakoutGameInstance)) _returnvalue_2)
      (Development|PrintText 0 "made new high score list" true true "(R=0.000000,G=0.660000,B=1.000000,A=1.000000)" 2e+01))))

(fn SaveHighScore
  (params (Difficulty :type E_Difficulties%20Enum :default "NewEnumerator0") (SaveGameObject :type Save%20Game%20Object%20Reference))
  (bind _returnvalue (CallFunction|GetDifficultySlot Difficulty))
  (SaveGame|SaveGametoSlot SaveGameObject (Utilities|String|EnumtoString _returnvalue)))

(fn LoadDifficultySlot
  (params (Difficulty :type E_Difficulties%20Enum :default "NewEnumerator0"))
  (bind _returnvalue (CallFunction|GetDifficultySlot Difficulty))
  (bind (_returnvalue_2 _success) (CallFunction|LoadSlot _returnvalue))
  (return _success _returnvalue_2))

(fn GetDifficultySlot
  (params (Difficulty :type E_Difficulties%20Enum :default "NewEnumerator0"))
  (switch Utilities|FlowControl|Switch|SwitchonE_Difficulties Difficulty
    (:NewEnumerator0
      (return (Utilities|Enum|LiteralenumE_Slots "NewEnumerator0")))
    (:NewEnumerator1
      (return (Utilities|Enum|LiteralenumE_Slots "NewEnumerator1")))
    (:NewEnumerator2
      (return (Utilities|Enum|LiteralenumE_Slots "NewEnumerator2")))))