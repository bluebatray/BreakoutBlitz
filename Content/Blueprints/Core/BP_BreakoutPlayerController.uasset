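; Player controller for a Breakout game that routes Enhanced Input to the paddle, ball launch and pause.
; On BeginPlay it adds the main mapping context and sets the initial game state.
; Horizontal input moves the possessed paddle, and pause changes the game state.
; The action key releases an attached ball through the game mode and starts its timer; otherwise it only prints a placeholder for a planned ability.
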(event Input|EnhancedActionEvents|EnhancedInputActionIA_HorizonatalMovement
  (params (ActionValue :type Float%20%28double-precision%29) (ElapsedSeconds :type Float%20%28double-precision%29) (TriggeredSeconds :type Float%20%28double-precision%29) (InputAction :type Input%20Action%20Object%20Reference :default "/Game/Input/IA_HorizonatalMovement.IA_HorizonatalMovement"))
  (CallFunction|HandleMove ActionValue))

(event Input|EnhancedActionEvents|EnhancedInputActionIA_ActionKey
  (params (ActionValue :type Boolean) (ElapsedSeconds :type Float%20%28double-precision%29) (TriggeredSeconds :type Float%20%28double-precision%29) (InputAction :type Input%20Action%20Object%20Reference :default "/Game/Input/IA_ActionKey.IA_ActionKey"))
  (:Completed
    (CallFunction|HandleActionKey)))

(event Input|EnhancedActionEvents|EnhancedInputActionIA_Pause
  (params (ActionValue :type Boolean) (ElapsedSeconds :type Float%20%28double-precision%29) (TriggeredSeconds :type Float%20%28double-precision%29) (InputAction :type Input%20Action%20Object%20Reference :default "/Game/Input/IA_Pause.IA_Pause"))
  (:Completed
    (CallFunction|UpdateGameState "NewEnumerator2")))

(event EventBeginPlay
  (CallFunction|AddInputContext)
  (CallFunction|UpdateGameState "NewEnumerator0"))

(fn ConstructionScript)

(fn AddInputContext
  ;[0 0 0] Adds Input mapping to game
  (Input|AddMappingContext (PlayerController|LocalPlayerSubsystems|GetEnhancedInputLocalPlayerSubsystem (Game|GetPlayerController 0)) "/Game/Input/IMC_MainContext.IMC_MainContext" 0 "(bIgnoreAllPressedKeysUntilRelease=True,bForceImmediately=False,bNotifyUserSettings=False)"))

(fn HandleMove
  (params (HorizontalMove :type Float%20%28double-precision%29))
  (bind _asbp_paddle (Utilities|Casting|CastToBP_Paddle (Pawn|GetControlledPawn)))
  (Default|Move _asbp_paddle HorizontalMove))

(fn HandleActionKey
  (bind _bp_paddle (CallFunction|GetPaddle))
  (if (Variables|/Game/Blueprints/BP_Paddle.BP_Paddle_C|GetbIsBallAttached _bp_paddle)
    (bind _bp_paddle_2 (CallFunction|GetPaddle))
    (Variables|/Game/Blueprints/BP_Paddle.BP_Paddle_C|SetbIsBallAttached _bp_paddle_2 false)
    (bind _breakout_game_mode (CallFunction|GetBreakoutGameMode))
    (Variables|/Game/Blueprints/Core/BP_BreakoutGameMode.BP_BreakoutGameMode_C|SetbIsUpdatingTimer _breakout_game_mode true)
    (Default|ShootBallfromPaddle (Variables|/Game/Blueprints/Core/BP_BreakoutGameMode.BP_BreakoutGameMode_C|GetBall _breakout_game_mode))
    (else
      ;[0.1388 1 0.1054] todo, ability
      (Development|PrintString "ball not attached to paddle" true true "(R=0.000000,G=0.660000,B=1.000000,A=1.000000)" 2e+01))))