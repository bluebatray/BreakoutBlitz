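; Player controller for a Breakout game that sets up input and shows the main menu.
; On BeginPlay it adds the IMC_MainContext Enhanced Input mapping context, then creates the main menu widget and adds it to the viewport.
; The horizontal movement input action is forwarded to the possessed BP_Paddle's Move function, doing nothing if the pawn is not a paddle.
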(event Input|EnhancedActionEvents|EnhancedInputActionIA_HorizonatalMovement
  (params (ActionValue :type Float%20%28double-precision%29) (ElapsedSeconds :type Float%20%28double-precision%29) (TriggeredSeconds :type Float%20%28double-precision%29) (InputAction :type Input%20Action%20Object%20Reference :default "/Game/Input/IA_HorizonatalMovement.IA_HorizonatalMovement"))
  (CallFunction|HandleMove ActionValue))

(event EventBeginPlay
  (CallFunction|AddInputContext)
  (bind _returnvalue (Game|ConstructObjectfromClass "/Game/Blueprints/BP_MainMenu.BP_MainMenu_C"))
  (UserInterface|Viewport|AddtoViewport _returnvalue 0))

(fn ConstructionScript)

(fn AddInputContext
  ;[0 0 0] Adds Input mapping to game
  (Input|AddMappingContext (PlayerController|LocalPlayerSubsystems|GetEnhancedInputLocalPlayerSubsystem (Game|GetPlayerController 0)) "/Game/Input/IMC_MainContext.IMC_MainContext" 0 "(bIgnoreAllPressedKeysUntilRelease=True,bForceImmediately=False,bNotifyUserSettings=False)"))

(fn HandleMove
  (params (HorizontalMove :type Float%20%28double-precision%29))
  (bind _asbp_paddle (Utilities|Casting|CastToBP_Paddle (Pawn|GetControlledPawn)))
  (Default|Move _asbp_paddle HorizontalMove))