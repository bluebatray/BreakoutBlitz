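; Game mode for a Breakout game, handling main menu, play, pause and game-over states with their widgets and input modes.
; Each level setup spawns a paddle-attached ball, applies difficulty settings and streams "NewLevel{N}"; a failed load counts as winning.
; Tagged blocks are counted after a short delay, and clearing them advances the level and banks its timer.
; Win, lose and pause dialogs take text from a data table, formatted with time and points.
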(event Custom|Count%20Level%20Time
  ;[0 0 0] Handle Time
  (Variables|GamePlay|SetbIsUpdatingTimer true)
  (bind _returnvalue (Utilities|Time|SetTimerbyEvent (EventDispatchers|CreateEvent :!event Custom|CountTime) (Variables|GamePlay|GetfTimerInterval) true))
  (Variables|GamePlay|SetLevelTimer _returnvalue))

(event Custom|StateChange_EnterMainMenu
  ;[0 0 0] States
  (CallFunction|SetInputMode true)
  (CallFunction|CreateandAddUserWidget "/Game/Blueprints/BP_MainMenu.BP_MainMenu_C" (Variables|Default|GetMainMenu)))

(event Custom|StateChange_EnterGameOver
  ;[0 0 0] States
  (CallFunction|SetInputMode true)
  (CallFunction|StopLevelTime)
  (bind _bpdialog (CallFunction|ShowWinLoseDialog))
  (EventDispatchers|AssignOnDialogConfirmed _bpdialog (EventDispatchers|CreateEvent :!event Custom|OnGameOverScreenClose))
  (Actor|DestroyActor (Variables|GamePlay|GetBall))
  (Widget|RemovefromParent (Variables|GamePlay|GetGameHud))
  (CallFunction|DestroyCurrentLevel))

(event Custom|OnGameOverScreenClose
  ;[0 0 0] States
  (Widget|RemovefromParent (Variables|GamePlay|GetGameHud))
  (CallFunction|UpdateGameState "NewEnumerator0"))

(event Custom|OnPauseScreenClose
  ;[0 0 0] States
  (CallFunction|SetInputMode false)
  (Game|SetGamePaused false))

(event Custom|StateChange_EnterPlayingGame
  ;[0 0 0] States
  (CallFunction|SetInputMode false)
  (CallFunction|CreateandAddUserWidget "/Game/Blueprints/BP_GameHud.BP_GameHud_C" (Variables|GamePlay|GetGameHud))
  (CallFunction|InitGame)
  (CallFunction|InitLevel)
  (CallFunction|SetupGame)
  (Utilities|CountBlocks)
  (Widget|RemovefromParent (Variables|Default|GetMainMenu)))

(event Custom|LevelEnded
  (CallFunction|DestroyCurrentLevel)
  (Actor|DestroyActor (Variables|GamePlay|GetBall))
  (Default|IncrementCurrentLevel (CallFunction|GetBreakoutGameInstance))
  (CallFunction|AddLevelTimetoTotal)
  (CallFunction|SetupGame)
  (Utilities|CountBlocks))

(event Custom|StateChange_EnterPause
  ;[0 0 0] States
  (CallFunction|SetInputMode true)
  (Game|SetGamePaused true)
  (bind _bpdialog (CallFunction|ShowDialog "NewEnumerator2"))
  (EventDispatchers|AssignOnDialogConfirmed _bpdialog (EventDispatchers|CreateEvent :!event Custom|OnPauseScreenClose)))

(event Custom|CountTime
  ;[0 0 0] Handle Time
  (Variables|GamePlay|SetfLevelTime (+ (Variables|GamePlay|GetfLevelTime) (Variables|GamePlay|GetfTimerInterval)))
  (Default|CallTimeUpdated))

(event Custom|Stop%20Level%20Time
  ;[0 0 0] Handle Time
  (Variables|GamePlay|SetbIsUpdatingTimer false)
  (Utilities|Time|ClearandInvalidateTimerbyHandle (Variables|GamePlay|GetLevelTimer)))

(fn ConstructionScript)

(fn SpawnBall
  (params (BallSpeed :type Float%20%28double-precision%29) (SpawnTransform :type Transform))
  (bind _bp_paddle (CallFunction|GetPaddle))
  (LocalVariables|SetBallAttachPoint (Variables|/Game/Blueprints/BP_Paddle.BP_Paddle_C|GetBallAttachPoint _bp_paddle))
  (bind _returnvalue (Game|SpawnActorfromClass "/Game/Blueprints/BP_Ball.BP_Ball_C" (Transformation|GetWorldTransform (LocalVariables|GetBallAttachPoint)) "AlwaysSpawn" "MultiplyWithRoot" 0 0))
  (Variables|GamePlay|SetBall _returnvalue)
  (Variables|/Game/Blueprints/BP_Ball.BP_Ball_C|SetBallSpeedMultiplier (Variables|GamePlay|GetBall) BallSpeed)
  (bind _returnvalue_2 (Transformation|AttachComponentToComponent (Variables|GamePlay|GetBall) (LocalVariables|GetBallAttachPoint) "None" "SnapToTarget" "SnapToTarget" "SnapToTarget" false))
  (bind _bp_paddle_2 (CallFunction|GetPaddle))
  (Variables|/Game/Blueprints/BP_Paddle.BP_Paddle_C|SetbIsBallAttached _bp_paddle_2 _returnvalue_2))

(fn SetupGame
  (Variables|GamePlay|SetfLevelTime 0.0)
  (Default|UpdateTime (Variables|GamePlay|GetGameHud))
  (bind _difficultyproperties (CallFunction|GetDifficultyMenuProperties (Utilities|String|StringToName (Utilities|String|EnumtoString (Variables|/Game/Blueprints/Core/BP_BreakoutGameInstance.BP_BreakoutGameInstance_C|GeteCurrentDifficulty (CallFunction|GetBreakoutGameInstance))))))
  (CallFunction|SpawnBall (.ballspeed _difficultyproperties))
  (bind _bp_paddle (CallFunction|GetPaddle))
  (Default|ChangePaddleSize _bp_paddle (.paddlelengthpercent _difficultyproperties))
  (CallFunction|LoadLevel))

(fn LoadLevel
  (CallFunction|StopLevelTime)
  (bind (_boutsuccess _returnvalue) (Class|LevelStreamingDynamic|LoadLevelInstance (Utilities|String|ToString(Text) (Utilities|Text|FormatText "NewLevel{CurrentLevel}" (Variables|/Game/Blueprints/Core/BP_BreakoutGameInstance.BP_BreakoutGameInstance_C|GetiCurrentLevel (CallFunction|GetBreakoutGameInstance)))) "0, 0, 0" "0, 0, 0" "" 0 false))
  (Variables|GamePlay|SetLoadedLevel _returnvalue)
  (if (not _boutsuccess)
    ;[0 0 0] No more levels, they win
    (CallFunction|UpdateGameState "NewEnumerator3")))

(fn DecrementBlocksLeft
  (Math|Integer|DecrementInt (Variables|GamePlay|GetiBlocksLeft)))

(fn HandleifBeatLevel
  (if (== (Variables|GamePlay|GetiBlocksLeft) 0)
    (CallFunction|LevelEnded)))

(fn SetEndGameText
  (params (BPDialog :type BP%20Dialog%20Object%20Reference) (eDialogScreen :type E_ScreenText%20Enum :default "E_DialogScreens_MAX"))
  (bind _returnvalue (Utilities|GetDataTableRow "/Game/Data/DT_ScreenText.DT_ScreenText" (Utilities|String|StringToName (Utilities|String|EnumtoString eDialogScreen)))
    (:then
      (bind _params (CallFunction|PopulateParams))
      (bind _textout (CallFunction|FormatTextwithParams (.text _returnvalue) _params))
      (Default|SetText BPDialog _textout))))

(fn ShowDialog
  (params (ScreenText :type E_ScreenText%20Enum :default "NewEnumerator0"))
  (bind _returnvalue (UserInterface|CreateWidget "/Game/Blueprints/BP_Dialog.BP_Dialog_C"))
  (CallFunction|SetEndGameText _returnvalue ScreenText)
  (UserInterface|Viewport|AddtoViewport _returnvalue 0)
  (return _returnvalue))

(fn PopulateParams
  (bind (_time _points) (CallFunction|GetEndGameParams))
  (return (Utilities|Array|MakeArray _time _points)))

(fn GetEndGameParams
  (bind _asbp_breakout_game_instance (CallFunction|GetBreakoutGameInstance))
  (bind _returnvalue (CallFunction|FormattoTime (Math|Float|Round (Variables|/Game/Blueprints/Core/BP_BreakoutGameInstance.BP_BreakoutGameInstance_C|GetfTotalGameTime _asbp_breakout_game_instance))))
  (return (Utilities|String|ToString(Text) _returnvalue) (Utilities|String|ToString(Integer) (Variables|/Game/Blueprints/Core/BP_BreakoutGameInstance.BP_BreakoutGameInstance_C|GetiCurrentPoints _asbp_breakout_game_instance))))

(fn InitLevel
  (Variables|GamePlay|SetbLostGame false))

(fn DestroyCurrentLevel
  (if (Utilities|IsValid (Variables|GamePlay|GetLoadedLevel))
    (Class|LevelStreaming|SetIsRequestingUnloadandRemoval (Variables|GamePlay|GetLoadedLevel) true)
    (Variables|GamePlay|SetiBlocksLeft 0)))

(fn SetInputMode
  (params (UI :type Boolean))
  (bind _returnvalue (Game|GetPlayerController 0))
  (bind _returnvalue_2 (Game|GetPlayerController 0))
  (if UI
    (Input|SetInputModeUIOnly _returnvalue 0 "DoNotLock" false)
    (Variables|/Script/Engine.PlayerController|SetbShowMouseCursor _returnvalue true)
    (else
      (Input|SetInputModeGameOnly _returnvalue_2 false)
      (Variables|/Script/Engine.PlayerController|SetbShowMouseCursor _returnvalue_2 false))))

(fn CreateandAddUserWidget
  (params (WidgetClass :type Object%20Class%20Reference) (WidgetRef :type User%20Widget%20Object%20Reference%20%28by%20ref%29))
  (bind _returnvalue (Game|ConstructObjectfromClass WidgetClass))
  (bind _asuser_widget (Utilities|Casting|CastToUserWidget _returnvalue))
  (|SetBy-RefVar WidgetRef _asuser_widget)
  (UserInterface|Viewport|AddtoViewport WidgetRef 0))

(fn ShowWinLoseDialog
  (if (Variables|GamePlay|GetbLostGame)
    (bind _bpdialog (CallFunction|ShowDialog "NewEnumerator3"))
    (return _bpdialog)
    (else
      (bind _bpdialog_2 (CallFunction|ShowDialog "NewEnumerator1"))
      (return _bpdialog_2))))