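; BP_BreakoutGameInstance is the Breakout game instance that tracks the current level, points and total game time.
; Small functions increment the level, accumulate time and add points looked up from a block's tier through GetBlockProperties.
; ResetAll restores the starting values, and both it and AddToPoints fire PointsChanged to signal score updates.
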(fn IncrementCurrentLevel
  (Math|Integer|IncrementInt (Variables|Default|GetiCurrentLevel)))

(fn AddtoPoints
  (params (Tier :type Integer))
  (bind _blockproperties (CallFunction|GetBlockProperties Tier))
  (Variables|Default|SetiCurrentPoints (+ (Variables|Default|GetiCurrentPoints) (.points _blockproperties)))
  (Default|CallPointsChanged))

(fn AddtoTotalGameTime
  (params (TimeToAdd :type Float%20%28double-precision%29))
  (Variables|Default|SetfTotalGameTime (+ TimeToAdd (Variables|Default|GetfTotalGameTime))))

(fn ResetAll
  (Variables|Default|SetfTotalGameTime 0.0)
  (Variables|Default|SetiCurrentPoints 0)
  (Variables|Default|SetiCurrentLevel 1)
  (Default|CallPointsChanged))