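; BP_Block is a breakable brick whose durability is tracked as a color Tier and a crack Level within that tier.
; Each OnBrickHit lowers Level, dropping a Tier and resetting Level when it runs out; a hit with Tier already below zero destroys the actor.
; Lookups by Tier and Level drive the Cube's color and crack-intensity material parameters, applied at construction, BeginPlay and on hits.
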(event Custom|OnBrickHit
  (CallFunction|HitBrick))

(event EventBeginPlay
  (CallFunction|SetTierColor)
  (CallFunction|SetLevelCrackage))

(event Collision|EventActorBeginOverlap
  (params (OtherActor :type Actor%20Object%20Reference)))

(event EventTick
  (params (DeltaSeconds :type Float%20%28single-precision%29)))

(fn ConstructionScript
  (CallFunction|SetTierColor)
  (CallFunction|SetLevelCrackage))

(fn HitBrick
  (if (< (Variables|Default|GetTier) 0)
    ;[1 1 1] dead
    (Actor|DestroyActor)
    (else
      (bind _tierupdated (CallFunction|DecrementLevel))
      (if _tierupdated
        (CallFunction|SetTierColor))
      (CallFunction|SetLevelCrackage))))

(fn DecrementLevel
  (if (<= (Variables|Default|GetLevel) 1)
    (Math|Integer|DecrementInt (Variables|Default|GetTier)
      (:%20%20
        (Variables|Default|SetLevel 3)
        (return true)))
    (else
      (Math|Integer|DecrementInt (Variables|Default|GetLevel)
        (:%20%20
          (return false))))))

(fn SetTierColor
  (Rendering|Material|SetVectorParameterValueonMaterials (Variables|Default|GetCube) "Color" (Math|Conversions|ToVector(LinearColor) (Math|Conversions|ToLinearColor(Color) (Utilities|Array|Get(acopy) (LocalVariables|GetColorLookup) (Variables|Default|GetTier))))))

(fn SetLevelCrackage
  (Rendering|Material|SetScalarParameterValueonMaterials (Variables|Default|GetCube) "CrackIntensity" (.Value (Utilities|Map|Find (LocalVariables|GetCrackIntensityLookup) (Variables|Default|GetLevel)))))